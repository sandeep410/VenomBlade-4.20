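; Corner trigger that turns the plane-constrained player and camera along a curved spline path.
; The construction script shapes the four-point spline from two pivots, the second angled by TurnRotation.
; While the player overlaps, a timeline samples the closest spline point to update the character's movement plane, back-plane normal and spring arm yaw.
; It also snaps actor location to the spline in XY, keeping Z.
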(event OnComponentBeginOverlap(CornerOverlap)
  (params (OverlappedComponent :type Primitive%20Component%20Object%20Reference) (OtherActor :type Actor%20Object%20Reference) (OtherComp :type Primitive%20Component%20Object%20Reference) (OtherBodyIndex :type Integer) (bFromSweep :type Boolean) (SweepResult :type Hit%20Result%20Structure%20%28by%20ref%29))
  (bind _returnvalue (Transformation|GetActorLocation))
  (bind _spline (Variables|Default|GetSpline))
  (bind _returnvalue_2 (Class|SplineComponent|FindRotationClosesttoWorldLocation _spline _returnvalue "World"))
  (bind _returnvalue_3 (Spline|FindLocationClosesttoWorldLocation _spline _returnvalue "World"))
  (bind _returnvalue_4 (Math|Vector|GetForwardVector _returnvalue_2))
  (bind (_x _y) (Math|Vector|BreakVector _returnvalue_3))
  (if (Components|ComponentHasTag OtherComp "Player")
    (bind _asfk_character (Utilities|Casting|CastToFK_Character (Components|GetOwner OtherComp)))
    (Variables|Default|Setfk_character _asfk_character)
    (Variables|Default|SetRef_SpringArm (Variables|/Game/Characters/Main/FK_Character.FK_Character_C|GetSpringArm1 _asfk_character))
    (Timeline|Timeline_SetNewRot Play
      (:Update
        (Variables|/Game/Characters/Main/FK_Character.FK_Character_C|SetBackPlaneNormal (Variables|Default|Getfk_character) _returnvalue_4)
        (Class|MovementComponent|SetPlaneConstraintfromVectors (Variables|/Script/Engine.Character|GetCharacterMovement (Variables|Default|Getfk_character)) _returnvalue_4 (Math|Vector|GetUpVector _returnvalue_2))
        (Transformation|SetActorLocation 0 (Math|Vector|MakeVector _x _y (.Z (Math|Vector|BreakVector _returnvalue))) false true)
        (Transformation|SetWorldRotation (Variables|Default|GetRef_SpringArm) (Math|Rotator|MakeRotator (.Roll (Math|Rotator|BreakRotator (Transformation|GetWorldRotation (Variables|Default|GetRef_SpringArm)))) (.Pitch (Math|Rotator|BreakRotator (Transformation|GetWorldRotation (Variables|Default|GetRef_SpringArm)))) (.Yaw (Math|Rotator|BreakRotator (Math|Rotator|CombineRotators _returnvalue_2 "0,-90.000000, 0")))) false false)))))

(event OnComponentEndOverlap(CornerOverlap)
  (params (OverlappedComponent :type Primitive%20Component%20Object%20Reference) (OtherActor :type Actor%20Object%20Reference) (OtherComp :type Primitive%20Component%20Object%20Reference) (OtherBodyIndex :type Integer))
  (bind _returnvalue (Transformation|GetActorLocation))
  (bind _spline (Variables|Default|GetSpline))
  (bind _ref_springarm (Variables|Default|GetRef_SpringArm))
  (bind _returnvalue_2 (Class|SplineComponent|FindRotationClosesttoWorldLocation _spline _returnvalue "World"))
  (bind _returnvalue_3 (Spline|FindLocationClosesttoWorldLocation _spline _returnvalue "World"))
  (bind _returnvalue_4 (Transformation|GetWorldRotation _ref_springarm))
  (bind (_roll _pitch) (Math|Rotator|BreakRotator _returnvalue_4))
  (bind _returnvalue_5 (Math|Vector|GetForwardVector _returnvalue_2))
  (bind (_x _y) (Math|Vector|BreakVector _returnvalue_3))
  (if (Components|ComponentHasTag OtherComp "Player")
    (Timeline|Timeline_SetNewRot Stop
      (:Update
        (Variables|/Game/Characters/Main/FK_Character.FK_Character_C|SetBackPlaneNormal (Variables|Default|Getfk_character) _returnvalue_5)
        (Class|MovementComponent|SetPlaneConstraintfromVectors (Variables|/Script/Engine.Character|GetCharacterMovement (Variables|Default|Getfk_character)) _returnvalue_5 (Math|Vector|GetUpVector _returnvalue_2))
        (Transformation|SetActorLocation 0 (Math|Vector|MakeVector _x _y (.Z (Math|Vector|BreakVector _returnvalue))) false true)
        (Transformation|SetWorldRotation _ref_springarm (Math|Rotator|MakeRotator _roll _pitch (.Yaw (Math|Rotator|BreakRotator (Math|Rotator|CombineRotators _returnvalue_2 "0,-90.000000, 0")))) false false)))))

(fn ConstructionScript
  (bind _turnpivot1 (Variables|Default|GetTurnPivot1))
  (bind _turnpivot2 (Variables|Default|GetTurnPivot2))
  (bind _relativelocation (Variables|/Script/Engine.SceneComponent|GetRelativeLocation _turnpivot2))
  (bind _relativelocation_2 (Variables|/Script/Engine.SceneComponent|GetRelativeLocation _turnpivot1))
  (bind _relativerotation (Variables|/Script/Engine.SceneComponent|GetRelativeRotation _turnpivot1))
  (bind _relativerotation_2 (Variables|/Script/Engine.SceneComponent|GetRelativeRotation _turnpivot2))
  (bind _returnvalue (Math|Vector|GetForwardVector _relativerotation_2))
  (bind _returnvalue_2 (Math|Vector|GetForwardVector _relativerotation))
  (bind _returnvalue_3 (* _returnvalue -2e+02))
  (Transformation|SetRelativeRotation (Variables|Default|GetTurnPivot2) (Math|Rotator|MakeRotator 0.0 0.0 (+ (Variables|Default|GetTurnRotation) 1.8e+02)) false false)
  (bind _output_get (Variables|Default|SetPathSpline (Variables|Default|GetSpline)))
  (Spline|SetLocationatSplinePoint _output_get 1 (+ _relativelocation_2 (* _returnvalue_2 -1e+02)) "Local" true)
  (Spline|SetTangentatSplinePoint _output_get 1 (* _returnvalue_2 2e+02) "Local" true)
  (Spline|SetLocationatSplinePoint _output_get 0 (+ _relativelocation_2 (* _returnvalue_2 -2e+02)) "Local" true)
  (Spline|SetTangentatSplinePoint _output_get 0 (* _returnvalue_2 2e+02) "Local" true)
  (Spline|SetLocationatSplinePoint _output_get 2 (+ _relativelocation (* _returnvalue -1e+02)) "Local" true)
  (Spline|SetTangentatSplinePoint _output_get 2 _returnvalue_3 "Local" true)
  (Spline|SetLocationatSplinePoint _output_get 3 (+ _relativelocation (* _returnvalue -2e+02)) "Local" true)
  (Spline|SetTangentatSplinePoint _output_get 3 _returnvalue_3 "Local" true))