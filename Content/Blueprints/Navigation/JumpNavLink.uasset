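; A nav link Blueprint that makes AI characters jump up or drop down when they reach its smart link.
; It compares mesh height to the destination, calling the character's AIJump for level or higher targets.
; For lower targets it launches the character along a fixed world -Y velocity, then resumes path following.
; An unconnected chain holds an alternative projectile-arc launch with a debug print and delay.
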(event EventSmartLinkReached
  (params (Agent :type Actor%20Object%20Reference) (Destination :type Vector%20%28by%20ref%29 :default "0, 0, 0"))
  (bind _asaibase_character (Utilities|Casting|CastToAIBaseCharacter Agent))
  (if (<= (.Z (Math|Vector|BreakVector (Transformation|GetWorldLocation (Variables|/Script/Engine.Character|GetMesh _asaibase_character)))) (.Z (Math|Vector|BreakVector Destination)))
    (Default|AIJump _asaibase_character Destination)
    (else
      (Character|LaunchCharacter _asaibase_character "0,-200.000000, 0" true false) ; jump down
      (Class|NavLinkProxy|ResumePathFollowing Agent))))

(fn ConstructionScript)