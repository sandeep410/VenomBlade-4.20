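; Game instance that handles saving and loading the player's game and keeps an index of save slot names.
; Init loads the SaveGameListe index from disk or creates a new one.
; SaveGame has FK_Character fill a new VenomSaveGame, writes it to its slot and records that name in the saved index.
; LoadGame reads a named slot, keeps it as CurrentSave across level travel and opens its stored level.
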(event Custom|SaveGame
  (bind _savelist (Variables|Default|GetSaveList))
  (bind _returnvalue (SaveGame|CreateSaveGameObject "/Game/Blueprints/SaveGame/VenomSaveGame.VenomSaveGame_C"))
  (bind _asfk_character (Utilities|Casting|CastToFK_Character (Game|GetPlayerCharacter 0)))
  (Default|SaveCharacter _asfk_character _returnvalue)
  (Development|PrintString (Utilities|String|ToString(Float) (Variables|/Game/Blueprints/SaveGame/VenomSaveGame.VenomSaveGame_C|GetCurrentHealth _returnvalue)))
  (SaveGame|SaveGametoSlot _returnvalue (Variables|/Game/Blueprints/SaveGame/VenomSaveGame.VenomSaveGame_C|GetSaveSlotName _returnvalue))
  (Utilities|Array|AddUnique (Variables|/Game/Blueprints/SaveGame/SaveGameListe.SaveGameListe_C|GetSaveNames _savelist) (Variables|/Game/Blueprints/SaveGame/VenomSaveGame.VenomSaveGame_C|GetSaveSlotName _returnvalue))
  (SaveGame|SaveGametoSlot _savelist (Variables|/Game/Blueprints/SaveGame/SaveGameListe.SaveGameListe_C|GetMainSlotName _savelist)))

(event Custom|LoadGame
  (params (SaveName :type String))
  (bind _returnvalue (SaveGame|LoadGamefromSlot SaveName))
  (bind _asvenom_save_game (Utilities|Casting|CastToVenomSaveGame _returnvalue))
  (Variables|Default|SetCurrentSave _asvenom_save_game)
  (Game|OpenLevel(byName) (Utilities|String|StringToName (Variables|/Game/Blueprints/SaveGame/VenomSaveGame.VenomSaveGame_C|GetCurrentLevelName _asvenom_save_game))))

(event EventInit
  (bind _returnvalue (SaveGame|CreateSaveGameObject "/Game/Blueprints/SaveGame/SaveGameListe.SaveGameListe_C"))
  (bind _returnvalue_2 (SaveGame|DoesSaveGameExist (Variables|/Game/Blueprints/SaveGame/SaveGameListe.SaveGameListe_C|GetMainSlotName _returnvalue) (Variables|/Game/Blueprints/SaveGame/SaveGameListe.SaveGameListe_C|GetUser _returnvalue)))
  (if _returnvalue_2
    (bind _returnvalue_3 (SaveGame|LoadGamefromSlot (Variables|/Game/Blueprints/SaveGame/SaveGameListe.SaveGameListe_C|GetMainSlotName _returnvalue) (Variables|/Game/Blueprints/SaveGame/SaveGameListe.SaveGameListe_C|GetUser _returnvalue)))
    (bind _assave_game_liste (Utilities|Casting|CastToSaveGameListe _returnvalue_3))
    (Variables|Default|SetSaveList _assave_game_liste)
    (else
      (bind _returnvalue_4 (SaveGame|CreateSaveGameObject "/Game/Blueprints/SaveGame/SaveGameListe.SaveGameListe_C"))
      (Variables|Default|SetSaveList _returnvalue_4))))